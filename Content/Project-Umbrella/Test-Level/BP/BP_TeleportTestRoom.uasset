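; Test-room teleporter pad Blueprint that prints debug readouts about the player's position relative to the Telepad.
; Each Tick runs through a one-second Delay, then transforms the player's location into the pad's relative-transform space and prints it, plus world X and an offset-adjusted relative X.
; When the player overlaps the outer teleport volume, it prints a collision message and a pad-extension status based on PadZ.
; Pad movement logic is unconnected, and no teleporting occurs.
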(event OnComponentBeginOverlap(TeleVol_Outer)
  (params (OverlappedComponent :type Primitive%20Component%20Object%20Reference) (OtherActor :type Actor%20Object%20Reference) (OtherComp :type Primitive%20Component%20Object%20Reference) (OtherBodyIndex :type Integer) (bFromSweep :type Boolean) (SweepResult :type Hit%20Result%20Structure%20%28by%20ref%29))
  (if (== OtherActor (Game|Player|GetPlayerPawn 0))
    (CallFunction|PadPlayerProxReact)))

(event Custom|PadPlayerProxReact
  (Development|PrintString "OUTER COLLISION TRIGGERED" true false "(R=0.989583,G=1.000000,B=0.979167,A=1.000000)" 0.5)
  (if (<= (Variables|Default|GetPad_Z) 3e+01)
    (Development|PrintString (|PadZMessage) true true "(R=0.000000,G=1.000000,B=0.991436,A=1.000000)" 1e+01)
    (else
      (Development|PrintString "Pad Fully Extended"))))

(event Collision|EventActorBeginOverlap
  (params (OtherActor :type Actor%20Object%20Reference)))

(event EventTick
  (params (DeltaSeconds :type Float%20%28single-precision%29))
  (Utilities|FlowControl|Delay 1.0)
  (Utilities|FlowControl|Sequence
    (:then_0
      (bind (_print_x _print_y _print_z_) (CallFunction|PadInverseXYZ))
      (|PrintXYZ _print_x _print_y _print_z_))
    (:then_1
      (Development|PrintString (Utilities|String|ToString(Float) (Variables|Default|GetPlayerX)) true true "(R=1.000000,G=0.022465,B=0.000000,A=1.000000)" 1.0)
      (Development|PrintString (Utilities|String|ToString(Float) (Variables|Default|GetRelativeX)) true true "(R=0.000000,G=0.668581,B=1.000000,A=1.000000)" 1.0))))

(fn ConstructionScript)

(fn PadInverseXYZ
  (bind _returnvalue (Game|Player|GetPlayerPawn 0))
  (bind _telepad (Variables|Default|GetTelepad))
  (bind _returnvalue_2 (Transformation|GetActorLocation _returnvalue))
  (bind _returnvalue_3 (Transformation|GetRelativeTransform _telepad))
  (bind _returnvalue_4 (Math|Transform|InverseTransformLocation _returnvalue_3 _returnvalue_2))
  (Variables|Default|SetPlayerX (.x (Transformation|GetActorLocation (Game|Player|GetPlayerPawn 0))))
  (Variables|Default|SetRelativeX (- (.x _returnvalue_4) (Variables|Default|GetPlayerProxRelativeOffset_X)))
  (return (Utilities|String|ToString(Float) (.x _returnvalue_4)) (Utilities|String|ToString(Float) (.y _returnvalue_4)) (Utilities|String|ToString(Float) (.z _returnvalue_4))))